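; BP_Bouncer continuously pulses the scale of every actor in its Actors list between a minimum and maximum multiple of its original size.
; On BeginPlay it caches each actor's initial scale, then a single timeline lerps all of them together.
; The timeline ping-pongs endlessly by reversing or restarting when finished, switching play rate so expanding and shrinking have separate speeds.
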(event `self.ReceiveBeginPlay`
  (for _array_element (`self.Actors`)
    (`KismetArrayLibrary.Array_Add` (`self.InitialScales`) (`self.GetActorScale3D` _array_element)))
  (bind (_direction _alpha) (`Timeline|ScaleTimeline` :!via `PlayFromStart` :!label _label)
    (:`Update`
      (for (_array_element_2 _array_index) (`self.Actors`)
        (bind _output (`|GetArrayItem` (`self.InitialScales`) _array_index))
        (`self.SetActorScale3D` _array_element_2 (`KismetMathLibrary.VLerp` (* _output (`self.MaxScale`)) (* _output (`self.MinScale`)) _alpha))))
    (:`Finished`
      (switch `ETimelineDirection` _direction
        (:`Forward`
          (`TimelineComponent.SetPlayRate` (`self.ScaleTimeline`) (`self.SpeedMinimizing`))
          (goto _label :!via `ReverseFromEnd`))
        (:`Backward`
          (`TimelineComponent.SetPlayRate` (`self.ScaleTimeline`) (`self.SpeedExpanding`))
          (goto _label :!via `PlayFromStart`))))))

(fn `MapVectorRangeClamped`
  (params (Value :type "Float (double-precision)") (Min :type "Vector Structure")))

(fn `UserConstructionScript`)