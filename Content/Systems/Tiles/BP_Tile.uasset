(event `self.ReceiveBeginPlay`
  (`self.GetDirectionalTiles`)
  (set `self.Tiles` (`|MakeArray` (`self.ForwardTile`) (`self.RightTile`) (`self.BackwardTile`) (`self.LeftTile`)))
  (set `self.Interactables` (`|MakeArray` (`self.ForwardInteractable`) (`self.RightInteractable`) (`self.BackwardInteractable`) (`self.LeftInteractable`)))
  (bind _asbp_player (cast `/Game/Systems/Player/BP_Player` (`GameplayStatics.GetPlayerPawn` 0)))
  (bind _output_get (set `self.As BP Player` _asbp_player))
  (add `/Game/Systems/Player/BP_Player.OnTurnCW` _output_get (delegate `OnTurnCWEvent`))
  (add `/Game/Systems/Player/BP_Player.OnTurnCCW` _output_get (delegate `OnTurnCCWEvent`)))

(event `OnTurnCWEvent`
  (`self.UpdatePlayerForwardTileCW`))

(event `OnTurnCCWEvent`
  (`self.UpdatePlayerForwardTileCCW`))

(fn `BuildBackward`
  (params (Class :type "/Game/Systems/Tiles/BP_Tile Class Reference"))
  (returns (BackwardTile :type "/Game/Systems/Tiles/BP_Tile Object Reference"))
  (bind (_min _max) (`StaticMeshComponent.GetLocalBounds` (`self.Plane`)))
  (bind _returnvalue_x (`KismetMathLibrary.BreakVector` (- _max _min)))
  (`/Engine/EditorBlueprintResources/StandardMacros.IsValid` (`self.BackwardTile`)
    (:`Is Valid`
      (return (`self.BackwardTile`)))
    (:`Is Not Valid`
      (bind _returnvalue (`|SpawnActorFromClass` Class (`KismetMathLibrary.MakeTransform` (- (`self.K2_GetActorLocation`) (`KismetMathLibrary.MakeVector` _returnvalue_x)) (`self.K2_GetActorRotation`)) "Undefined" "MultiplyWithRoot" null false null))
      (bind _output_get (set `self.BackwardTile` _returnvalue))
      (return _output_get))))

(fn `BuildForward`
  (params (Class :type "/Game/Systems/Tiles/BP_Tile Class Reference"))
  (returns (Output_Get :type "/Game/Systems/Tiles/BP_Tile Object Reference"))
  (bind (_min _max) (`StaticMeshComponent.GetLocalBounds` (`self.Plane`)))
  (bind _returnvalue_x (`KismetMathLibrary.BreakVector` (- _max _min)))
  (`/Engine/EditorBlueprintResources/StandardMacros.IsValid` (`self.ForwardTile`)
    (:`Is Valid`
      (return (`self.ForwardTile`)))
    (:`Is Not Valid`
      (bind _returnvalue (`|SpawnActorFromClass` Class (`KismetMathLibrary.MakeTransform` (+ (`self.K2_GetActorLocation`) (`KismetMathLibrary.MakeVector` _returnvalue_x)) (`self.K2_GetActorRotation`)) "Undefined" "MultiplyWithRoot" null false null))
      (bind _output_get (set `self.ForwardTile` _returnvalue))
      (return _output_get))))

(fn `BuildLeft`
  (params (Class :type "/Game/Systems/Tiles/BP_Tile Class Reference"))
  (returns (Output_Get :type "/Game/Systems/Tiles/BP_Tile Object Reference"))
  (bind (_min _max) (`StaticMeshComponent.GetLocalBounds` (`self.Plane`)))
  (bind (_returnvalue_x _returnvalue_y) (`KismetMathLibrary.BreakVector` (- _max _min)))
  (`/Engine/EditorBlueprintResources/StandardMacros.IsValid` (`self.LeftTile`)
    (:`Is Valid`
      (return (`self.LeftTile`)))
    (:`Is Not Valid`
      (bind _returnvalue (`|SpawnActorFromClass` Class (`KismetMathLibrary.MakeTransform` (- (`self.K2_GetActorLocation`) (`KismetMathLibrary.MakeVector` 0.0 _returnvalue_y)) (`self.K2_GetActorRotation`)) "Undefined" "MultiplyWithRoot" null false null))
      (bind _output_get (set `self.LeftTile` _returnvalue))
      (return _output_get))))

(fn `BuildRight`
  (params (Class :type "/Game/Systems/Tiles/BP_Tile Class Reference"))
  (returns (Output_Get :type "/Game/Systems/Tiles/BP_Tile Object Reference"))
  (bind (_min _max) (`StaticMeshComponent.GetLocalBounds` (`self.Plane`)))
  (bind (_returnvalue_x _returnvalue_y) (`KismetMathLibrary.BreakVector` (- _max _min)))
  (`/Engine/EditorBlueprintResources/StandardMacros.IsValid` (`self.RightTile`)
    (:`Is Valid`
      (return (`self.RightTile`)))
    (:`Is Not Valid`
      (bind _returnvalue (`|SpawnActorFromClass` Class (`KismetMathLibrary.MakeTransform` (+ (`self.K2_GetActorLocation`) (`KismetMathLibrary.MakeVector` 0.0 _returnvalue_y)) (`self.K2_GetActorRotation`)) "Undefined" "MultiplyWithRoot" null false null))
      (bind _output_get (set `self.RightTile` _returnvalue))
      (return _output_get))))

(fn `FindHoleGroundTile`
  (bind _returnvalue (`self.K2_GetActorLocation`))
  (bind _outhit (`KismetSystemLibrary.LineTraceSingle` :`Start` _returnvalue :`End` (- _returnvalue (0.0 0.0 1000.0)) :`TraceChannel` "TraceTypeQuery1" :`DrawDebugType` "ForDuration"))
  (bind (_bblockinghit _binitialoverlap _time _distance _location _impactpoint _normal _impactnormal _physmat _hitactor) (`GameplayStatics.BreakHitResult` _outhit))
  (if (== (`GameplayStatics.GetObjectClass` _hitactor) "BP_Tile_C")
    (bind _asbp_tile (cast `/Game/Systems/Tiles/BP_Tile` _hitactor))
    (set `self.holeGroundTile` _asbp_tile)))

(fn `GetDirection`
  (params (Direction :type "/Game/Systems/Tiles/E_TileDirection Enum" :default "NewEnumerator0"))
  (returns (`AsBP Tile` :type "/Game/Systems/Tiles/BP_Tile Object Reference"))
  (bind _returnvalue (`self.K2_GetActorRotation`))
  (bind _returnvalue_2 (`SceneComponent.K2_GetComponentLocation` (`self.Box`)))
  (bind _outhit (`KismetSystemLibrary.LineTraceSingle` :`Start` _returnvalue_2 :`End` (+ _returnvalue_2 (* (select `/Game/Systems/Tiles/E_TileDirection` (`local.Direction`) :`NewEnumerator0` (`KismetMathLibrary.GetForwardVector` _returnvalue) :`NewEnumerator1` (`KismetMathLibrary.NegateVector` (`KismetMathLibrary.GetForwardVector` _returnvalue)) :`NewEnumerator2` (`KismetMathLibrary.NegateVector` (`KismetMathLibrary.GetRightVector` _returnvalue)) :`NewEnumerator3` (`KismetMathLibrary.GetRightVector` _returnvalue)) (* (`BoxComponent.GetScaledBoxExtent` (`self.Box`)) 2.0))) :`TraceChannel` "TraceTypeQuery1" :`DrawDebugType` "ForDuration" :`DrawTime` 1.0))
  (return (cast `/Game/Systems/Tiles/BP_Tile` (`.HitActor` (`GameplayStatics.BreakHitResult` _outhit)) :!pure true)))

(fn `GetDirectionalTiles`
  (`|ExecutionSequence`
    (:`then_0`
      (bind _asbp_tile (`self.GetDirection` "NewEnumerator0"))
      (set `self.ForwardTile` _asbp_tile))
    (:`then_1`
      (bind _asbp_tile_2 (`self.GetDirection` "NewEnumerator1"))
      (set `self.BackwardTile` _asbp_tile_2))
    (:`then_2`
      (bind _asbp_tile_3 (`self.GetDirection` "NewEnumerator2"))
      (set `self.LeftTile` _asbp_tile_3))
    (:`then_3`
      (bind _asbp_tile_4 (`self.GetDirection` "NewEnumerator3"))
      (set `self.RightTile` _asbp_tile_4))))

(fn `UpdatePlayerForwardTileCCW`
  (bind _as_bp_player (`self.As BP Player`))
  (bind _output_get (set `/Game/Systems/Player/BP_Player.ForwardTile` (`|GetArrayItem` (`/Game/Systems/Tiles/BP_Tile.Tiles` (`/Game/Systems/Player/BP_Player.CurrentTile` _as_bp_player)) (`/Game/Systems/Player/BP_Player.forwardTileIndex` _as_bp_player)) (`self.As BP Player`)))
  (`KismetSystemLibrary.PrintString` (`KismetSystemLibrary.GetDisplayName` _output_get)))

(fn `UpdatePlayerForwardTileCW`
  (bind _as_bp_player (`self.As BP Player`))
  (bind _output_get (set `/Game/Systems/Player/BP_Player.ForwardTile` (`|GetArrayItem` (`/Game/Systems/Tiles/BP_Tile.Tiles` (`/Game/Systems/Player/BP_Player.CurrentTile` _as_bp_player)) (`/Game/Systems/Player/BP_Player.forwardTileIndex` _as_bp_player)) (`self.As BP Player`)))
  (`KismetSystemLibrary.PrintString` (`KismetSystemLibrary.GetDisplayName` _output_get)))

(fn `UserConstructionScript`
  (`self.GetDirectionalTiles`)
  (if (`self.isHole`)
    (`self.FindHoleGroundTile`)))