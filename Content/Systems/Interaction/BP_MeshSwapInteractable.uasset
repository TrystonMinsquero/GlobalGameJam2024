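; Interactable actor that swaps its mesh between an initial and a swapped static mesh when the player interacts with it.
; The construction script applies the initial mesh, and Interact flips the state, updates the mesh, then calls an empty PlaySound hook and the parent Interact.
; DoOnce makes the swap one-way and blanks the prompt afterward, though it still reports usable; otherwise the prompt follows the current state.
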(fn `GetInteractText`
  (returns (ReturnValue :type Text) (Usable :type Boolean))
  (return (select `bool` (`self.bAlreadySwapped`) :`false` (`self.InitialText`) :`true` (select `bool` (`self.bDoOnce`) :`false` (`self.SwappedText`))) true))

(fn `Interact`
  (returns (ReturnValue :type Boolean))
  (if (not (and (`self.bAlreadySwapped`) (`self.bDoOnce`)))
    (set `self.bAlreadySwapped` (not (`self.bAlreadySwapped`)))
    (`self.SwapMesh`)
    (`self.PlaySound`)
    (bind _returnvalue (`parent.Interact`))
    (return _returnvalue)))

(fn `PlaySound`)

(fn `SwapMesh`
  (`StaticMeshComponent.SetStaticMesh` (`self.Mesh`) (select `bool` (`self.bAlreadySwapped`) :`false` (`self.InitialMesh`) :`true` (`self.SwappedMesh`))))

(fn `UserConstructionScript`
  (`parent.UserConstructionScript`)
  (`StaticMeshComponent.SetStaticMesh` (`self.Mesh`) (`self.InitialMesh`)))