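; BP_PickupItem is an interactable inventory pickup, identified by a VariableId flag that records whether it has been taken.
; Interact works only if the item is untaken and no other item is held; it sets the flag, refreshes the mesh and turns off the light, with special music for HasCat.
; SetMesh derives the mesh from that flag and GameMode inventory settings, at construction and on Reset, which clears the flag.
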(event `/Game/Systems/Interaction/BPI_Resetable.Reset`
  (`/Game/Systems/GameFramework/BP_GlobalFL.SetVariable` (`self.VariableId`))
  (`self.SetMesh`))

(fn `GetInteractText`
  (returns (ReturnValue :type Text) (Usable :type Boolean))
  (return (select `bool` (`/Game/Systems/GameFramework/BP_GlobalFL.GetVariable` (`self.VariableId`)) :`false` (select `bool` (`/Game/Systems/GameFramework/BP_GlobalFL.IsHoldingInventoryItem`) :`false` (`self.CanPickupText`) :`true` (`self.Can'tPickupText`))) (not (`/Game/Systems/GameFramework/BP_GlobalFL.IsHoldingInventoryItem`))))

(fn `Interact`
  (returns (ReturnValue :type Boolean))
  (if (not (or (`/Game/Systems/GameFramework/BP_GlobalFL.GetVariable` (`self.VariableId`)) (`/Game/Systems/GameFramework/BP_GlobalFL.IsHoldingInventoryItem`)))
    (`/Game/Systems/GameFramework/BP_GlobalFL.SetVariable` (`self.VariableId`) true)
    (`self.SetMesh`)
    (`LightComponent.SetIntensity` (`self.PointLight`) 0.0)
    (if (== (`self.VariableId`) "HasCat")
      (`/Game/Systems/GameFramework/BP_GlobalFL.PlayMusic` "/Game/Audio/Music/ST_Cat_Theme.ST_Cat_Theme"))
    (bind _returnvalue (`parent.Interact`))
    (return _returnvalue)))

(fn `SetMesh`
  (bind _returnvalue (`/Game/Systems/GameFramework/BP_GlobalFL.GetGameMode`))
  (`/Engine/EditorBlueprintResources/StandardMacros.IsValid` (`StaticMeshComponent.StaticMesh` (`self.Mesh`))
    (:`Is Valid`
      (`/Engine/EditorBlueprintResources/StandardMacros.IsValid` _returnvalue
        (:`Is Valid`
          (`StaticMeshComponent.SetStaticMesh` (`self.Mesh`) (select `bool` (`/Game/Systems/GameFramework/BP_GlobalFL.GetVariable` (`self.VariableId`)) :`false` (`.Mesh_8_6D1A528B43FA5B5857803381235B2758` (break `/Game/Systems/Player/F_PlayerFacingMesh` (`BlueprintMapLibrary.Map_Find` (`/Game/Systems/GameFramework/PDA_GameSettings.InventoryVariables` (`/Game/Systems/GameFramework/BP_GameMode.Settings` _returnvalue)) (`self.VariableId`)))))))))))

(fn `UserConstructionScript`
  (`parent.UserConstructionScript`)
  (`self.SetMesh`))