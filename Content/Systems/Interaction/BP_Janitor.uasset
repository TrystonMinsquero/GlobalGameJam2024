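; BP_Janitor is an interactable janitor object that has powered and unplugged states.
; SetMesh picks the default or unplugged static mesh from the Powered flag, though nothing in this Blueprint calls it.
; Interact and GetInteractText defer to the parent only while powered.
; When unpowered, the prompt is blank and interaction skips the parent logic, yet GetInteractText still reports it as usable.
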(fn `GetInteractText`
  (returns (ReturnValue :type Text) (Usable :type Boolean))
  (bind _returnvalue (`parent.GetInteractText`))
  (return (select `bool` (`self.bPowered`) :`true` _returnvalue) true))

(fn `Interact`
  (returns (ReturnValue :type Boolean))
  (if (`self.bPowered`)
    (bind _returnvalue (`parent.Interact`))
    (return _returnvalue)))

(fn `Set Mesh`
  (if (`self.bPowered`)
    (`StaticMeshComponent.SetStaticMesh` (`self.StaticMesh`) "/Game/Art/Assets/Bathroom/Janitor/Janitor_Default.Janitor_Default")
    (else
      (`StaticMeshComponent.SetStaticMesh` (`self.StaticMesh`) "/Game/Art/Assets/Bathroom/Janitor/Janitor_Unplugged.Janitor_Unplugged"))))

(fn `UserConstructionScript`
  (`parent.UserConstructionScript`))