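; AI controller for NPCs that runs branching dialogue, starting a conversation by running the supplied dialogue behavior tree and showing the player HUD's dialogue widget.
; Lines display text and play positional audio at the pawn for their duration; response menus add options afterward and broadcast the selected choice.
; CanMoveOn and GetChoice expose line and choice state.
; Leave requests end the conversation, stopping tree logic and any current sound.
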(event `/Game/Systems/DialogueSystem/BPI_DialogueController.StartConversation`
  (params (DialogueTree :type "BehaviorTree Object Reference"))
  (`Widget.SetVisibility` (`self.GetDialogueWidget`) "Visible")
  (`self.RunBehaviorTree` DialogueTree))

(event `/Game/Systems/DialogueSystem/BPI_DialogueController.EndConversation`
  (`Widget.SetVisibility` (`self.GetDialogueWidget`) "Hidden")
  (`BrainComponent.StopLogic` (`self.BrainComponent`) "")
  (`/Engine/EditorBlueprintResources/StandardMacros.IsValid` (`self.CurrentSound`)
    (:`Is Valid`
      (`AudioComponent.Stop` (`self.CurrentSound`)))
    (:`Is Not Valid`
      _))
  (set `self.CurrentSound` null))

(event `self.ReceiveBeginPlay`
  (bind _returnvalue (`self.GetDialogueWidget`))
  (`KismetSystemLibrary.DelayUntilNextTick`)
  (`Widget.SetVisibility` _returnvalue "Hidden")
  (add `/Game/UI/HUD/Dialogue/WBP_DialogueMenu.LeaveRequested` _returnvalue (delegate `OnLeaveRequested`)))

(event `OnLeaveRequested`
  (`self.EndConversation`))

(event `/Game/Systems/DialogueSystem/BPI_DialogueController.ShowResponseMenu`
  (params (ChoiceId :type Name) (Dialogue :type Text) (Audio :type "SoundBase Object Reference") (ReponseOptions :type "Array of Text (by ref)") (HideIndexes :type "Array of Integer (by ref)"))
  (set `self.CurrentChoice` ChoiceId)
  (add `/Game/UI/HUD/Dialogue/WBP_DialogueMenu.OnResponseSelected` (`self.GetDialogueWidget`) (delegate `/Game/Systems/DialogueSystem/BPI_DialogueController.OnResponseSelected`))
  (`self.StartLine` Dialogue Audio)
  (`KismetSystemLibrary.Delay` (`SoundBase.Duration` Audio))
  (`/Game/UI/HUD/Dialogue/WBP_DialogueMenu.AddResponses` (`self.GetDialogueWidget`) ReponseOptions HideIndexes))

(event `/Game/Systems/DialogueSystem/BPI_DialogueController.OnResponseSelected`
  (params (Index :type Integer))
  (set `self.Index` Index)
  (remove `/Game/UI/HUD/Dialogue/WBP_DialogueMenu.OnResponseSelected` (`self.GetDialogueWidget`) (delegate `/Game/Systems/DialogueSystem/BPI_DialogueController.OnResponseSelected`))
  (`self.ResponseSelected` (`self.CurrentChoice`) (`self.Index`))
  (set `self.CurrentChoice` "None"))

(event `/Game/Systems/DialogueSystem/BPI_DialogueController.StartLine`
  (params (Text :type Text) (Audio :type "SoundBase Object Reference"))
  (set `self.bPlayingDialogue` true)
  (`/Game/UI/HUD/Dialogue/WBP_DialogueMenu.AddDialogue` (`self.GetDialogueWidget`) Text)
  (bind _returnvalue (`GameplayStatics.SpawnSoundAtLocation` Audio (`self.K2_GetActorLocation` (`self.K2_GetPawn`)) (struct) 1.0 1.0 0.0 null null))
  (set `self.CurrentSound` _returnvalue)
  (`KismetSystemLibrary.Delay` (`SoundBase.Duration` Audio))
  (set `self.bPlayingDialogue` false)
  (set `self.CurrentSound` null))

(fn `CanMoveOn`
  (returns (ReturnValue :type Boolean))
  (return (and (not (`self.bPlayingDialogue`)) (== (`self.CurrentChoice`) "None"))))

(fn `GetChoice`
  (returns (ChoiceId :type Name) (Index :type Integer))
  (return (`self.CurrentChoice`) (`self.Index`)))

(fn `GetDialogueWidget`
  (returns (ReturnValue :type "/Game/UI/HUD/Dialogue/WBP_DialogueMenu Object Reference"))
  (`/Engine/EditorBlueprintResources/StandardMacros.IsValid` (`self.DialogueWidget`)
    (:`Is Valid`
      _)
    (:`Is Not Valid`
      (bind _asbp_player (cast `/Game/Systems/Player/BP_Player` (`GameplayStatics.GetPlayerPawn` 0))
        (:`then`
          (set `self.DialogueWidget` (`/Game/UI/HUD/WBP_HUD.WBP_DialogueMenu` (`/Game/Systems/Player/BP_Player.HUD` _asbp_player))))
        (:`CastFailed`
          _))))
  (return (`self.DialogueWidget`)))

(fn `UserConstructionScript`)