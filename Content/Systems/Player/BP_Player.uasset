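; Player actor for tile-based movement: steps between linked tiles, turns in 90-degree increments and interacts with whatever the current tile holds ahead.
; ForwardTileIndex tracks facing and selects the neighbour tile and interactable, whose prompt Tick sends to the HUD.
; A timeline lerps each step and drops the player through hole tiles, while Tick lerps rotation toward DesiredRotation.
; DoOnce gates with timers enforce cooldowns; the timeline-based turn path is disconnected.
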(event `CheckForwardKey`
  (if (and (`self.canMoveForwards`) (`KismetSystemLibrary.IsValid` (`|GetArrayItem` (`/Game/Systems/Tiles/BP_Tile.Tiles` (`self.CurrentTile`)) (`self.forwardTileIndex`))))
    (if (`/Game/Systems/Tiles/BP_Tile.canMoveTo` (`|GetArrayItem` (`/Game/Systems/Tiles/BP_Tile.Tiles` (`self.CurrentTile`)) (`self.forwardTileIndex`)))
      (if (not (or (`|GetInputActionValue`) (`|GetInputActionValue`)))
        (`self.StartMoving`)))))

(event `StartMoving`
  (bind _arrow (`/Game/Systems/Tiles/BP_Tile.Arrow` (`|GetArrayItem` (`/Game/Systems/Tiles/BP_Tile.Tiles` (`self.CurrentTile`)) (`self.forwardTileIndex`)))
    (:`then`
      (bind (_direction _alpha) (`Timeline|TakeStep` :!via `PlayFromStart` :!label _label)
        (:`Update`
          (`self.K2_SetActorLocation` (`KismetMathLibrary.VLerp` (`self.K2_GetActorLocation`) (`SceneComponent.K2_GetComponentLocation` _arrow) (* _alpha (`/Game/Systems/Player/PDA_Player.MoveToSpeed` (`self.Data`))))))
        (:`Finished`
          (bind _forwardtile (`self.ForwardTile`)
            (:`then`
              (bind _output_get (set `self.CurrentTile` _forwardtile))
              (`self.OnTileEntered` _output_get)
              (`/Game/Systems/Tiles/BP_Tile.OnPlayerEnter` _output_get)
              (set `self.ForwardTile` (`|GetArrayItem` (`/Game/Systems/Tiles/BP_Tile.Tiles` (`self.CurrentTile`)) (`self.forwardTileIndex`)))
              (if (`/Game/Systems/Tiles/BP_Tile.isHole` (`self.CurrentTile`))
                (bind (_direction_2 _alpha_2) (`Timeline|Fall` :!via `PlayFromStart`)
                  (:`Update`
                    (`self.K2_SetActorLocation` (`KismetMathLibrary.VLerp` (`self.K2_GetActorLocation`) (`SceneComponent.K2_GetComponentLocation` (`/Game/Systems/Tiles/BP_Tile.Arrow` (`/Game/Systems/Tiles/BP_Tile.holeGroundTile` (`self.CurrentTile`)))) _alpha_2)))
                  (:`Finished`
                    (bind _output_get_2 (set `self.CurrentTile` (`/Game/Systems/Tiles/BP_Tile.holeGroundTile` (`self.CurrentTile`))))
                    (`/Game/Systems/Tiles/BP_Tile.OnPlayerEnter` _output_get_2)
                    (set `self.ForwardTile` (`|GetArrayItem` (`/Game/Systems/Tiles/BP_Tile.Tiles` (`self.CurrentTile`)) (`self.forwardTileIndex`)))))))
            (:`else`)))))
    (:`else`
      (goto _label :!via `Stop`))))

(event `CheckTurnKey`
  (if (`self.bTurnCW`)
    (`self.TurnCW`)
    (set `self.bTurnCW` false)
    (elif (`self.bTurnCCW`)
      (`self.TurnCCW`)
      (set `self.bTurnCCW` false))))

(event `StartTurning`
  (bind _returnvalue_x (`KismetMathLibrary.BreakVector2D` (`|GetInputActionValue`)))
  (bind _returnvalue_x_2 (`KismetMathLibrary.BreakVector2D` (`|GetInputActionValue`)))
  (bind _yaw (.yaw (`self.StartRotation`)))
  (bind _yaw_2 (.yaw (`self.StartRotation`)))
  (bind (_direction _alpha) (`Timeline|DoTurn` :!via `PlayFromStart`)
    (:`Update`
      (if (> _returnvalue_x_2 0.0)
        (bind (_returnvalue_roll _returnvalue_pitch _returnvalue_yaw) (`KismetMathLibrary.BreakRotator` (`KismetMathLibrary.RLerp` (`KismetMathLibrary.MakeRotator` 0.0 0.0 _yaw) (`KismetMathLibrary.MakeRotator` 0.0 0.0 (+ _yaw 90.0)) _alpha)))
        (bind _returnvalue (`KismetMathLibrary.MakeRotator` 0.0 0.0 _returnvalue_yaw))
        (`self.K2_SetActorRotation` _returnvalue)
        (elif (< _returnvalue_x_2 0.0)
          (bind (_returnvalue_roll_2 _returnvalue_pitch_2 _returnvalue_yaw_2) (`KismetMathLibrary.BreakRotator` (`KismetMathLibrary.RLerp` (`KismetMathLibrary.MakeRotator` 0.0 0.0 _yaw_2) (`KismetMathLibrary.MakeRotator` 0.0 0.0 (+ _yaw_2 -90.0)) _alpha)))
          (bind _returnvalue_2 (`KismetMathLibrary.MakeRotator` 0.0 0.0 _returnvalue_yaw_2))
          (`self.K2_SetActorRotation` _returnvalue_2))))
    (:`Finished`
      (`self.StopTurning`)
      (if (> _returnvalue_x 0.0)
        (set `self.StartRotation` _returnvalue)
        (elif (< _returnvalue_x 0.0)
          (set `self.StartRotation` _returnvalue_2))))))

(event `self.ReceiveBeginPlay`
  (bind _asplayer_controller (cast `PlayerController` (`self.GetController`)))
  (`EnhancedInputSubsystemInterface.AddMappingContext` (pcsubsystem `EnhancedInputLocalPlayerSubsystem` _asplayer_controller) (`self.PlayerIMC`) 0 (struct))
  (`self.ResetPlayer` (`/Game/Systems/GameFramework/BP_GameMode.StartTile` (`/Game/Systems/GameFramework/BP_GlobalFL.GetGameMode`)))
  (`self.CreateWidgets`))

(event `EnhancedInput|/Game/Systems/Player/Input/Actions/IA_Interact`
  (params (ActionValue :type Boolean) (ElapsedSeconds :type "Float (double-precision)") (TriggeredSeconds :type "Float (double-precision)") (InputAction :type "InputAction Object Reference" :default "/Game/Systems/Player/Input/Actions/IA_Interact.IA_Interact"))
  (:`Triggered`
    (message `/Game/Systems/Interaction/BPI_Interactable.Interact` (`|GetArrayItem` (`/Game/Systems/Tiles/BP_Tile.Interactables` (`self.CurrentTile`)) (`self.forwardTileIndex`)))))

(event `EnhancedInput|/Game/Systems/Player/Input/Actions/IA_Forward`
  (params (ActionValue :type Boolean) (ElapsedSeconds :type "Float (double-precision)") (TriggeredSeconds :type "Float (double-precision)") (InputAction :type "InputAction Object Reference" :default "/Game/Systems/Player/Input/Actions/IA_Forward.IA_Forward"))
  (:`Triggered`
    (`/Engine/EditorBlueprintResources/StandardMacros.DoOnce` false :!label _label_2
      (:`Completed`
        (`|ExecutionSequence`
          (:`then_0`
            (`self.CheckForwardKey`))
          (:`then_1`
            (bind _returnvalue (`KismetSystemLibrary.K2_SetTimerDelegate` (delegate `ResetMoveCD`) (`/Game/Systems/Player/PDA_Player.MovementCooldown` (`self.Data`))))
            (set `self.moveCDhandle` _returnvalue)))))))

(event `ResetMoveCD`
  (goto _label_2 :!via `Reset`))

(event `EnhancedInput|/Game/Systems/Player/Input/Actions/IA_TurnCCW`
  (params (ActionValue :type Boolean) (ElapsedSeconds :type "Float (double-precision)") (TriggeredSeconds :type "Float (double-precision)") (InputAction :type "InputAction Object Reference" :default "/Game/Systems/Player/Input/Actions/IA_TurnCCW.IA_TurnCCW"))
  (:`Triggered`
    (`/Engine/EditorBlueprintResources/StandardMacros.DoOnce` false :!label _label_3
      (:`Completed`
        (`|ExecutionSequence`
          (:`then_0`
            (`self.TurnCCW`))
          (:`then_1`
            (`KismetSystemLibrary.K2_SetTimerDelegate` (delegate `ResetTurnCD`) (`/Game/Systems/Player/PDA_Player.TurnCooldown` (`self.Data`)) :!label _label_4)))))))

(event `ResetTurnCD`
  (`|ExecutionSequence`
    (:`then_0`
      (goto _label_3 :!via `Reset`))
    (:`then_1`
      (goto _label_5 :!via `Reset`))))

(event `EnhancedInput|/Game/Systems/Player/Input/Actions/IA_TurnCW`
  (params (ActionValue :type Boolean) (ElapsedSeconds :type "Float (double-precision)") (TriggeredSeconds :type "Float (double-precision)") (InputAction :type "InputAction Object Reference" :default "/Game/Systems/Player/Input/Actions/IA_TurnCW.IA_TurnCW"))
  (:`Triggered`
    (`/Engine/EditorBlueprintResources/StandardMacros.DoOnce` false :!label _label_5
      (:`Completed`
        (`|ExecutionSequence`
          (:`then_0`
            (`self.TurnCW`))
          (:`then_1`
            (goto _label_4)))))))

(event `self.ReceiveTick`
  (params (DeltaSeconds :type "Float (single-precision)"))
  (bind _returnvalue (`self.K2_GetActorRotation`))
  (bind _desiredrotation (`self.DesiredRotation`))
  (`|ExecutionSequence`
    (:`then_0`
      (bind _returnvalue_2 (message `/Game/Systems/Interaction/BPI_Interactable.GetInteractText` (`|GetArrayItem` (`/Game/Systems/Tiles/BP_Tile.Interactables` (`self.CurrentTile`)) (`self.forwardTileIndex`))))
      (`self.SetInteractableText` _returnvalue_2))
    (:`then_1`
      (if (`|GetInputActionValue`)
        (set `self.canMoveForwards` true)
        (else
          (`|ExecutionSequence`
            (:`then_0`
              (if (`|GetInputActionValue`)
                (set `self.bTurnCW` true)))
            (:`then_1`
              (if (`|GetInputActionValue`)
                (set `self.bTurnCCW` true)))))))
    (:`then_2`
      (if (!= _returnvalue _desiredrotation)
        (`self.K2_SetActorRotation` (`KismetMathLibrary.RLerp` _returnvalue _desiredrotation (`/Game/Systems/Player/PDA_Player.TurnToSpeed` (`self.Data`)) true))))))

(fn `CreateWidgets`
  (bind _returnvalue (`|CreateWidget` "/Game/UI/HUD/WBP_HUD.WBP_HUD_C" (`GameplayStatics.GetPlayerController` 0)))
  (bind _output_get (set `self.HUD` _returnvalue))
  (`UserWidget.AddToViewport` _output_get 0))

(fn `LineTraceFromCamera`
  (returns (OutHit :type "HitResult Structure") (ReturnValue :type Boolean))
  (bind _camera (`self.Camera`))
  (bind _returnvalue (`SceneComponent.K2_GetComponentLocation` _camera))
  (bind (_outhit _returnvalue_2) (`KismetSystemLibrary.LineTraceSingleForObjects` :`Start` _returnvalue :`End` (+ _returnvalue (* (`SceneComponent.GetForwardVector` _camera) 300.0)) :`ObjectTypes` (`|MakeArray` "ObjectTypeQuery1" "ObjectTypeQuery2" :!type "EObjectTypeQuery Enum") :`DrawDebugType` "ForOneFrame"))
  (return _outhit _returnvalue_2))

(fn `ResetPlayer`
  (params (Start :type "/Game/Systems/Tiles/BP_Tile Object Reference"))
  (bind _arrow (`/Game/Systems/Tiles/BP_Tile.Arrow` (`self.CurrentTile`)))
  (set `self.CurrentTile` Start)
  (bind _output_get (set `self.DesiredRotation` (`SceneComponent.K2_GetComponentRotation` _arrow)))
  (`self.K2_SetActorLocation` (`SceneComponent.K2_GetComponentLocation` _arrow))
  (bind _output_get_2 (set `self.forwardTileIndex` (`KismetMathLibrary.Min` (`KismetMathLibrary.Round` (/ (.yaw _output_get) 90.0)) (- (`KismetArrayLibrary.Array_Length` (`/Game/Systems/Tiles/BP_Tile.Tiles` (`self.CurrentTile`))) 1))))
  (set `self.ForwardTile` (`|GetArrayItem` (`/Game/Systems/Tiles/BP_Tile.Tiles` (`self.CurrentTile`)) _output_get_2))
  (`self.OnTileEntered` (`self.CurrentTile`)))

(fn `SetInteractableText`
  (params (Text :type Text))
  (`/Game/UI/HUD/WBP_InteractPrompt.SetInteractableText` (`/Game/UI/HUD/WBP_HUD.WBP_InteractPrompt` (`self.HUD`)) Text))

(fn `StopMoving`)

(fn `StopTurning`)

(fn `TurnCCW`
  (bind _forwardtileindex (`self.forwardTileIndex`))
  (set `self.DesiredRotation` (`KismetMathLibrary.NormalizedDeltaRotator` (`self.DesiredRotation`) (`KismetMathLibrary.MakeRotator` 0.0 0.0 90.0)))
  (set `self.forwardTileIndex` (select `bool` (> _forwardtileindex 0) :`false` 3 :`true` (- _forwardtileindex 1)))
  (`self.OnTurnCCW`))

(fn `TurnCW`
  (bind _forwardtileindex (`self.forwardTileIndex`))
  (set `self.DesiredRotation` (`KismetMathLibrary.ComposeRotators` (`self.DesiredRotation`) (`KismetMathLibrary.MakeRotator` 0.0 0.0 90.0)))
  (set `self.forwardTileIndex` (select `bool` (< _forwardtileindex 3) :`true` (+ _forwardtileindex 1)))
  (`self.OnTurnCW`))

(fn `UserConstructionScript`)