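; Music manager component that switches between 2D songs with sequential fades, resuming each song from its tracked playback position.
; PlayMusic queues a different song, and the next game mode TimeUpdated tick starts the transition.
; A map lazily caches each song's audio component and elapsed time, advanced every tick for the current song.
; Fade out, delay and fade in each last half the game mode's time step.
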(event `self.ReceiveBeginPlay`
  (add `/Game/Systems/GameFramework/BP_GameMode.TimeUpdated` (`/Game/Systems/GameFramework/BP_GlobalFL.GetGameMode`) (delegate `OnTimeUpdated`)))

(event `OnTimeUpdated`
  (`self.IncrementCurrentSongTime`)
  (if (`self.bPlayNewSong`)
    (set `self.bPlayNewSong` false)
    (`self.StartSongTransition` (`self.SongToPlay`))
    (set `self.SongToPlay` null)))

(event `Play Music`
  (params (Song :type "SoundBase Object Reference"))
  (if (!= Song (`self.CurrentSong`))
    (set `self.SongToPlay` Song)
    (set `self.bPlayNewSong` true)))

(event `StartSongTransition`
  (params (NewSong :type "SoundBase Object Reference"))
  (bind _returnvalue (`self.GetFadeDuration`))
  (bind (_soundcomponent _currenttime) (break `/Game/Systems/MusicManager/F_SongInfo` (`self.GetSoundInfo` NewSong)))
  (bind _soundcomponent_2 (break `/Game/Systems/MusicManager/F_SongInfo` (`self.GetSoundInfo` (`self.CurrentSong`))))
  (`/Engine/EditorBlueprintResources/StandardMacros.IsValid` _soundcomponent_2
    (:`Is Valid`
      (`AudioComponent.FadeOut` _soundcomponent_2 _returnvalue 0.0 "Linear"))
    (:`Is Not Valid`
      _))
  (`KismetSystemLibrary.Delay` _returnvalue)
  (set `self.CurrentSong` NewSong)
  (`/Engine/EditorBlueprintResources/StandardMacros.IsValid` _soundcomponent
    (:`Is Valid`
      (`AudioComponent.FadeIn` _soundcomponent (`self.GetFadeDuration`) 1.0 _currenttime "Linear"))))

(fn `GetFadeDuration`
  (returns (ReturnValue :type "Float (double-precision)"))
  (return (/ (`/Game/Systems/GameFramework/PDA_GameSettings.TimeStepDurationInSeconds` (`/Game/Systems/GameFramework/BP_GameMode.Settings` (`/Game/Systems/GameFramework/BP_GlobalFL.GetGameMode`))) 2.0)))

(fn `GetSoundInfo`
  (params (Song :type "SoundBase Object Reference"))
  (returns (ReturnValue :type "/Game/Systems/MusicManager/F_SongInfo Structure"))
  (bind (_value _returnvalue) (`BlueprintMapLibrary.Map_Find` (`self.CurrentSongs`) (`local.Song`)))
  (`/Engine/EditorBlueprintResources/StandardMacros.IsValid` Song
    (:`Is Valid`
      (if _returnvalue :!label _label
        (return _value)
        (else
          (bind _returnvalue_2 (`GameplayStatics.CreateSound2D` (`local.Song`) 1.0 1.0 0.0 null))
          (`BlueprintMapLibrary.Map_Add` (`self.CurrentSongs`) (`local.Song`) (make `/Game/Systems/MusicManager/F_SongInfo` _returnvalue_2))
          (goto _label))))
    (:`Is Not Valid`
      (return (make `/Game/Systems/MusicManager/F_SongInfo` null)))))

(fn `IncrementCurrentSongTime`
  (bind (_soundcomponent _currenttime) (break `/Game/Systems/MusicManager/F_SongInfo` (`self.GetSoundInfo` (`self.CurrentSong`))))
  (`/Engine/EditorBlueprintResources/StandardMacros.IsValid` _soundcomponent
    (:`Is Valid`
      (`BlueprintMapLibrary.Map_Add` (`self.CurrentSongs`) (`self.CurrentSong`) (make `/Game/Systems/MusicManager/F_SongInfo` _soundcomponent (+ _currenttime (`/Game/Systems/GameFramework/PDA_GameSettings.TimeStepDurationInSeconds` (`/Game/Systems/GameFramework/BP_GameMode.Settings` (`/Game/Systems/GameFramework/BP_GlobalFL.GetGameMode`)))))))))