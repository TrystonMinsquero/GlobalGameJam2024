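; BP_Door is a one-time interactable door that gates movement between connecting tiles in a tile-based movement system.
; It listens to the player's tile-entered event, blocking all connecting tiles while the player stands on one, until the door is swapped.
; Unlocking can require specific player tiles and a boolean key variable, which drive the prompt text.
; Interacting runs the parent's logic, refreshes tile access and optionally clears the key.
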(event `self.ReceiveBeginPlay`
  (`parent.ReceiveBeginPlay`)
  (bind _asbp_player (cast `/Game/Systems/Player/BP_Player` (`GameplayStatics.GetPlayerPawn` 0)))
  (bind _output_get (set `self.player` _asbp_player))
  (add `/Game/Systems/Player/BP_Player.OnTileEntered` _output_get (delegate `OnTileEntered`)))

(event `OnTileEntered`
  (params (TileEntered :type "/Game/Systems/Tiles/BP_Tile Object Reference"))
  (for _array_element (`self.ConnectingTiles`)
    (set `/Game/Systems/Tiles/BP_Tile.canMoveTo` (or (`self.bAlreadySwapped`) (not (`KismetArrayLibrary.Array_Contains` (`self.ConnectingTiles`) TileEntered))) _array_element)))

(fn `CanUnlock`
  (returns (ReturnValue :type Boolean))
  (bind _unlocktiles (`self.UnlockTiles`))
  (return (and (or (`KismetArrayLibrary.Array_IsEmpty` _unlocktiles) (`KismetArrayLibrary.Array_Contains` _unlocktiles (`/Game/Systems/Player/BP_Player.CurrentTile` (`self.player`)))) (or (== (`self.KeyVariableId`) "None") (`/Game/Systems/GameFramework/BP_GlobalFL.GetVariable` (`self.KeyVariableId`))))))

(fn `GetInteractText`
  (returns (ReturnValue :type Text) (Usable :type Boolean))
  (bind _returnvalue (`self.CanUnlock`))
  (if (`self.bAlreadySwapped`)
    (return "" false)
    (else
      (return (select `bool` _returnvalue :`false` (`self.Locked Text`) :`true` (`self.Unlocked Text`)) _returnvalue))))

(fn `Interact`
  (returns (ReturnValue :type Boolean))
  (if (`self.CanUnlock`)
    (bind _returnvalue (`parent.Interact`))
    (`self.OnTileEntered` (`/Game/Systems/Player/BP_Player.CurrentTile` (`self.player`)))
    (if (`self.ClearKey`)
      (`/Game/Systems/GameFramework/BP_GlobalFL.SetVariable` (`self.KeyVariableId`))
      (return _returnvalue))))

(fn `UserConstructionScript`
  (`parent.UserConstructionScript`))