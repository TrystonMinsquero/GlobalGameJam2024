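; Game mode that runs a timed reset loop, ending each run with a conversation with a hidden Death NPC.
; A looping timer counts down, then blacks out the screen, cuts off any current conversation and starts Death's dialogue.
; When that conversation ends, StartGame resets interface-tagged actors, the player to the start tile, and non-persistent variables.
; It also stores boolean variables, broadcasting changes and updating the player's held-item mesh for inventory entries.
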(event `self.ReceiveBeginPlay`
  (bind _asbp_player (cast `/Game/Systems/Player/BP_Player` (`GameplayStatics.GetPlayerPawn` 0)))
  (set `self.Player` _asbp_player)
  (`WidgetBlueprintLibrary.SetInputMode_GameAndUIEx` (`GameplayStatics.GetPlayerController` 0) null)
  (`self.GetStartTile`)
  (`self.StartGame`))

(event `OnTalkedToDeathNPC`
  (remove `/Game/Systems/Interaction/BP_NPC.ConversationEnded` (`self.GetDeathNPC`) (delegate `OnTalkedToDeathNPC`))
  (`self.StartGame`))

(event `StartDialogueLate`
  (`KismetSystemLibrary.Delay` 1.0)
  (`/Game/Systems/Interaction/BP_NPC.Interact` (`self.GetDeathNPC`)))

(fn `AsGameMode`
  (returns (ReturnValue :type "/Game/Systems/GameFramework/BP_GameMode Object Reference"))
  (return self))

(fn `ClearVariables`
  (bind _keys (`BlueprintMapLibrary.Map_Keys` (`self.Variables`)))
  (for _array_element _keys
    (if (not (`BlueprintSetLibrary.Set_Contains` (`/Game/Systems/GameFramework/PDA_GameSettings.PersistantVariables` (`self.Settings`)) _array_element))
      (`BlueprintMapLibrary.Map_Add` (`self.Variables`) _array_element))))

(fn `GetDeathNPC`
  (returns (ReturnValue :type "/Game/Systems/Interaction/BP_Death_NPC Object Reference"))
  (`/Engine/EditorBlueprintResources/StandardMacros.IsValid` (`self.DeathNPC`)
    (:`Is Valid`
      (return (`self.DeathNPC`)))
    (:`Is Not Valid`
      (bind _returnvalue (`|SpawnActorFromClass` "/Game/Systems/Interaction/BP_Death_NPC.BP_Death_NPC_C" (`KismetMathLibrary.MakeTransform` (0.0 0.0 0.0)) "Undefined" "MultiplyWithRoot" null null))
      (`self.SetActorHiddenInGame` _returnvalue true)
      (bind _output_get (set `self.DeathNPC` _returnvalue))
      (return _output_get))))

(fn `GetStartTile`
  (bind _outactors (`GameplayStatics.GetAllActorsOfClassWithTag` "/Game/Systems/Tiles/BP_Tile.BP_Tile_C" "StartTile"))
  (set `self.StartTile` (`|GetArrayItem` _outactors)))

(fn `SetVariable`
  (params (VariableId :type Name) (Value :type Boolean))
  (bind _mesh (`/Game/Systems/Player/BP_Player.Mesh` (`self.Player`)))
  (bind (_value _returnvalue) (`BlueprintMapLibrary.Map_Find` (`/Game/Systems/GameFramework/PDA_GameSettings.InventoryVariables` (`self.Settings`)) (`local.VariableId`)))
  (bind (_mesh_2 _positionoffset _rotationoffset) (break `/Game/Systems/Player/F_PlayerFacingMesh` _value))
  (`BlueprintMapLibrary.Map_Add` (`self.Variables`) VariableId Value)
  (`self.VariableSet` VariableId Value)
  (if _returnvalue
    (`StaticMeshComponent.SetStaticMesh` _mesh (select `bool` (`local.Value`) :`true` _mesh_2))
    (`SceneComponent.K2_SetRelativeLocationAndRotation` _mesh _positionoffset _rotationoffset false false)))

(fn `Start Dialogue with Death NPC`
  (bind _currentnpc (`/Game/Systems/Player/BP_Player.currentNPC` (`self.Player`)))
  (if (not (`self.bGameOver`))
    (set `self.bGameOver` true)
    (`/Game/Systems/GameFramework/BP_GlobalFL.Set Timer Paused` true)
    (`/Game/Systems/GameFramework/BP_GlobalFL.PlayMusic` null)
    (`self.TimeUpdated`)
    (`/Game/UI/HUD/WBP_HUD.SetBlackScreen` (`/Game/Systems/Player/BP_Player.HUD` (`self.Player`)) true false)
    (`/Engine/EditorBlueprintResources/StandardMacros.IsValid` _currentnpc
      (:`Is Valid`
        (message `/Game/Systems/DialogueSystem/BPI_DialogueController.EndConversation` (`AIBlueprintHelperLibrary.GetAIController` _currentnpc)))
      (:`Is Not Valid`
        _))
    (add `/Game/Systems/Interaction/BP_NPC.ConversationEnded` (`self.GetDeathNPC`) (`|CreateDelegate` :!event `OnTalkedToDeathNPC`))
    (`self.StartDialogueLate`)))

(fn `StartGame`
  (bind _hud (`/Game/Systems/Player/BP_Player.HUD` (`self.Player`)))
  (set `self.bGameOver` false)
  (`self.ClearVariables`)
  (bind _outactors (`GameplayStatics.GetAllActorsWithInterface` "/Game/Systems/Interaction/BPI_Resetable.BPI_Resetable_C"))
  (for _array_element _outactors
    (message `/Game/Systems/Interaction/BPI_Resetable.Reset` _array_element))
  (`/Engine/EditorBlueprintResources/StandardMacros.IsValid` _hud
    (:`Is Valid`
      (`/Game/UI/HUD/WBP_HUD.SetBlackScreen` _hud false false))
    (:`Is Not Valid`
      _))
  (`/Game/Systems/Player/BP_Player.ResetPlayer` (`self.Player`) (`self.StartTile`))
  (`KismetSystemLibrary.K2_ClearAndInvalidateTimerHandle` (`self.GameTimer`))
  (set `self.TimeRemaining` (`/Game/Systems/GameFramework/PDA_GameSettings.TimeTillReset` (`self.Settings`)))
  (bind _returnvalue (`KismetSystemLibrary.K2_SetTimer` null "UpdateTime" (`/Game/Systems/GameFramework/PDA_GameSettings.TimeStepDurationInSeconds` (`self.Settings`)) true))
  (set `self.GameTimer` _returnvalue))

(fn `UpdateTime`
  (`/Engine/EditorBlueprintResources/StandardMacros.DecrementInt` (`self.TimeRemaining`)
    (:`  `
      (`self.TimeUpdated`)
      (if (<= (`self.TimeRemaining`) 0)
        (`self.Start Dialogue with Death NPC`)))))

(fn `UserConstructionScript`)