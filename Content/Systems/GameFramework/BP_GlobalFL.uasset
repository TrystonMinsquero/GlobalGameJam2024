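; Global Blueprint function library that gives access to shared game mode state: variables, the game timer and music.
; Wrappers resolve the game mode through GetGameMode to set or read ID-keyed variables, read remaining time, pause the timer and play songs.
; CheckVariables evaluates a list of boolean variables by all/any true/false rules, passing when the list is empty.
; IsHoldingInventoryItem reports whether any inventory variable from the game mode's settings is true.
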(fn `CheckVariables`
  (params (CheckType :type "/Game/Systems/DialogueSystem/E_AnyOrAll Enum" :default "NewEnumerator0") (Variables :type "Array of Name"))
  (returns (ReturnValue :type Boolean))
  (if (`KismetArrayLibrary.Array_IsNotEmpty` Variables)
    (for _array_element (`local.Variables`)
      (switch `/Game/Systems/DialogueSystem/E_AnyOrAll` (`local.CheckType`)
        (:`NewEnumerator0`
          (bind _returnvalue (`self.GetVariable` _array_element (`local.__WorldContext`)))
          (if (not _returnvalue)
            (return false)))
        (:`NewEnumerator1`
          (if _returnvalue
            (return true)))
        (:`NewEnumerator2`
          (if _returnvalue
            (return false)))
        (:`NewEnumerator3`
          (if (not _returnvalue)
            (return true)))))
    (switch `/Game/Systems/DialogueSystem/E_AnyOrAll` "NewEnumerator0"
      (:`NewEnumerator0`
        _)
      (:`NewEnumerator1`
        (return false))
      (:`NewEnumerator2`
        _)
      (:`NewEnumerator3`
        (return false)))
    (return true)
    (else
      (return true))))

(fn `GetGameMode`
  (returns (ReturnValue :type "/Game/Systems/GameFramework/BP_GameMode Object Reference"))
  (bind _returnvalue (message `/Game/Systems/GameFramework/BPI_GameMode.AsGameMode` (`GameplayStatics.GetGameMode` (`local.__WorldContext`))))
  (return _returnvalue))

(fn `GetGlobalTimeRemaining`
  (returns (Time :type Integer))
  (return (`/Game/Systems/GameFramework/BP_GameMode.TimeRemaining` (`self.GetGameMode` (`local.__WorldContext`)))))

(fn `GetVariable`
  (params (VariableId :type Name))
  (returns (ReturnValue :type Boolean))
  (return (`BlueprintMapLibrary.Map_Find` (`/Game/Systems/GameFramework/BP_GameMode.Variables` (`self.GetGameMode` (`local.__WorldContext`))) VariableId)))

(fn `IsHoldingInventoryItem`
  (returns (ReturnValue :type Boolean))
  (bind _keys (`BlueprintMapLibrary.Map_Keys` (`/Game/Systems/GameFramework/PDA_GameSettings.InventoryVariables` (`/Game/Systems/GameFramework/BP_GameMode.Settings` (`self.GetGameMode` (`local.__WorldContext`))))))
  (for _array_element _keys
    (if (`self.GetVariable` _array_element (`local.__WorldContext`))
      (return true)))
  (return false))

(fn `PlayMusic`
  (params (Song :type "SoundBase Object Reference"))
  (`/Game/Systems/MusicManager/AC_MusicManager.Play Music` (`/Game/Systems/GameFramework/BP_GameMode.AC_MusicManager` (`self.GetGameMode` (`local.__WorldContext`))) Song))

(fn `Set Timer Paused`
  (params (Paused :type Boolean :default true))
  (bind ___worldcontext (`local.__WorldContext`))
  (bind _gametimer (`/Game/Systems/GameFramework/BP_GameMode.GameTimer` (`self.GetGameMode` (`local.__WorldContext`))))
  (if Paused
    (`KismetSystemLibrary.K2_PauseTimerHandle` ___worldcontext _gametimer)
    (else
      (`KismetSystemLibrary.K2_UnPauseTimerHandle` ___worldcontext _gametimer))))

(fn `SetVariable`
  (params (VariableId :type Name) (Value :type Boolean))
  (`/Game/Systems/GameFramework/BP_GameMode.SetVariable` (`self.GetGameMode` (`local.__WorldContext`)) VariableId Value))