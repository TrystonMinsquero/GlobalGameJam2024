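; BP_Chef is the chef character in the interaction system, changing its static mesh in response to the GoblinKey game variable.
; On BeginPlay it registers with the game mode's variable-set notification and binds to its conversation-ended event.
; Setting GoblinKey true switches the mesh to Chef_Cat, and a conversation ending while it is true switches it to Chef_Cat_HMN.
; A choice-checking event is an unused stub.
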(event `HMMMMM`
  ;[1 1 1] on convo ended check variable
  (if (`/Game/Systems/GameFramework/BP_GlobalFL.GetVariable` "GoblinKey")
    (`StaticMeshComponent.SetStaticMesh` (`self.StaticMesh`) "/Game/Art/Assets/Kitchen/Chef_n_Cat/Chef_Cat_HMN.Chef_Cat_HMN")))

(event `self.ReceiveBeginPlay`
  (`parent.ReceiveBeginPlay`)
  (add `/Game/Systems/GameFramework/BP_GameMode.VariableSet` (`/Game/Systems/GameFramework/BP_GlobalFL.GetGameMode`) (delegate `CheckVariable`))
  (add `self.ConversationEnded` (delegate `HMMMMM`)))

(event `CheckVariable`
  (params (VariableId :type Name) (Value :type Boolean))
  ;[1 1 1] Checks variable when any are set
  (if (and (== VariableId "GoblinKey") Value)
    (`StaticMeshComponent.SetStaticMesh` (`self.StaticMesh`) "/Game/Art/Assets/Kitchen/Chef_n_Cat/Chef_Cat.Chef_Cat")))

(event `Hummmmmmmmm`
  (params (ChoiceId :type Name) (Index :type Integer))
  ;[1 1 1] Not used, but can be used to check index and id
  (if (and (== ChoiceId "Chef_01") (== Index 2))
    _))

(fn `UserConstructionScript`
  (`parent.UserConstructionScript`))