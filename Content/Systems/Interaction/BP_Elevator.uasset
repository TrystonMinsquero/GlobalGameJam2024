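; BP_Elevator is an interactable elevator that teleports the player to its TeleportTile through BP_Player's ResetPlayer once it has power.
; An unpowered elevator flagged TurnsOnPower switches power on when used, and its prompt text reflects each state.
; Powering up also powers the linked OtherElevator, swapping both meshes' materials and raising their light intensity, though these visuals update only when that link is valid.
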(fn `GetInteractText`
  (returns (ReturnValue :type Text) (Usable :type Boolean))
  (return (select `bool` (`self.bHasPower`) :`false` (select `bool` (`self.bTurnsOnPower`) :`false` "Needs power!" :`true` "Press E to turn on power." :!type "Text") :`true` "Press E to use elevator") (`self.bHasPower`)))

(fn `Interact`
  (returns (ReturnValue :type Boolean))
  (if (`self.bHasPower`)
    (`self.Teleport`)
    (return true)
    (elif (`self.bTurnsOnPower`)
      (`self.TurnOnPower`)
      (return true))))

(fn `Teleport`
  (bind _asbp_player (cast `/Game/Systems/Player/BP_Player` (`GameplayStatics.GetPlayerPawn` 0)))
  (`/Game/Systems/Player/BP_Player.ResetPlayer` _asbp_player (`self.TeleportTile`)))

(fn `TurnOnPower`
  (bind _otherelevator (`self.OtherElevator`))
  (set `self.bHasPower` true)
  (`/Engine/EditorBlueprintResources/StandardMacros.IsValid` _otherelevator
    (:`Is Valid`
      (set `/Game/Systems/Interaction/BP_Elevator.bHasPower` true _otherelevator)
      (`PrimitiveComponent.SetMaterial` (`self.Mesh`) 1 "/Game/Art/Materials/MI_Elevator.MI_Elevator")
      (`PrimitiveComponent.SetMaterial` (`/Game/Systems/Interaction/BP_Elevator.Mesh` _otherelevator) 1 "/Game/Art/Materials/MI_Elevator.MI_Elevator")
      (`LightComponent.SetIntensity` (`self.e`) 1000.0)
      (`LightComponent.SetIntensity` (`/Game/Systems/Interaction/BP_Elevator.e` _otherelevator) 1000.0))))

(fn `UserConstructionScript`
  (`parent.UserConstructionScript`)
  (if (`self.bHasPower`)
    (`LightComponent.SetIntensity` (`self.e`) 1000.0)
    (`PrimitiveComponent.SetMaterial` (`self.Mesh`) 1 "/Game/Art/Materials/MI_Elevator.MI_Elevator")))